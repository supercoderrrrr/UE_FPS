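; First-person shooter player Blueprint handling Enhanced Input movement, look, sprint, aim and firing.
; Tick aligns the arm to control rotation, derives Idle/Walk/Run/Aim state, sets walk speed from it, and prints that speed.
; Aiming overrides forward-only sprint, lowers look sensitivity and interpolates FOV inward; a looping timer restores it on release.
; BeginPlay spawns BP_VIRTUS on the arm; firing, blocked while running or dead, delegates to that weapon.
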(event Custom|OutFOV
  (bind _camera (Variables|Default|GetCamera))
  (bind _fieldofview (Variables|/Script/Engine.CameraComponent|GetFieldOfView _camera))
  (Camera|SetFieldOfView _camera (Math|Interpolation|FInterpTo _fieldofview (Variables|Default|GetDefaultFOV) (Utilities|Time|GetWorldDeltaSeconds) 8.0))
  (if (Math|Float|NearlyEqual(Float) _fieldofview (Variables|Default|GetDefaultFOV) 0.1)
    (Utilities|Time|ClearandInvalidateTimerbyHandle (Variables|Default|GetOutFOVHandle))))

(event Input|EnhancedActionEvents|EnhancedInputActionIA_Move
  (params (ActionValue :type Vector%202D%20Structure) (ElapsedSeconds :type Float%20%28double-precision%29) (TriggeredSeconds :type Float%20%28double-precision%29) (InputAction :type Input%20Action%20Object%20Reference :default "/Game/Code/Player/System/Input/IA_Move.IA_Move"))
  (bind (_x _y) (Math|Vector2D|BreakVector2D ActionValue))
  (:Triggered
    (bind _output_get (Variables|Default|SetMove%20X _x))
    (Pawn|Input|AddMovementInput (Math|Vector|GetForwardVector (Math|Rotator|MakeRotator 0.0 0.0 (.yaw (Pawn|GetControlRotation :!class /Script/Engine.Pawn)))) _output_get false)
    (bind _output_get_2 (Variables|Default|SetMove%20Y _y))
    (Pawn|Input|AddMovementInput (Math|Vector|GetRightVector (Math|Rotator|MakeRotator 0.0 0.0 (.yaw (Pawn|GetControlRotation :!class /Script/Engine.Pawn)))) _output_get_2 false))
  (:Completed
    (Variables|Default|SetMove%20X 0.0) ; 键盘松开后的执行引脚
    (Variables|Default|SetMove%20Y 0.0)))

(event Input|EnhancedActionEvents|EnhancedInputActionIA_Look
  (params (ActionValue :type Vector%202D%20Structure) (ElapsedSeconds :type Float%20%28double-precision%29) (TriggeredSeconds :type Float%20%28double-precision%29) (InputAction :type Input%20Action%20Object%20Reference :default "/Game/Code/Player/System/Input/IA_Look.IA_Look"))
  (bind (_x _y) (Math|Vector2D|BreakVector2D ActionValue))
  (Pawn|Input|AddControllerYawInput (* _x (CallFunction|UpdateScopeSensitivity) (Variables|Default|GetMouseSensitivity)))
  (Pawn|Input|AddControllerPitchInput (* _y (CallFunction|UpdateScopeSensitivity) (Variables|Default|GetMouseSensitivity))))

(event Input|EnhancedActionEvents|EnhancedInputActionIA_Run
  (params (ActionValue :type Boolean) (ElapsedSeconds :type Float%20%28double-precision%29) (TriggeredSeconds :type Float%20%28double-precision%29) (InputAction :type Input%20Action%20Object%20Reference :default "/Game/Code/Player/System/Input/IA_Run.IA_Run"))
  (:Triggered
    (Variables|Default|SetWant%20To%20Run true))
  (:Completed
    (Variables|Default|SetWant%20To%20Run false)))

(event Input|EnhancedActionEvents|EnhancedInputActionIA_Aim
  (params (ActionValue :type Boolean) (ElapsedSeconds :type Float%20%28double-precision%29) (TriggeredSeconds :type Float%20%28double-precision%29) (InputAction :type Input%20Action%20Object%20Reference :default "/Game/Code/Player/System/Input/IA_Aim.IA_Aim"))
  (bind _camera (Variables|Default|GetCamera))
  (:Triggered
    (Variables|Default|SetWant%20To%20Aim true)
    (Camera|SetFieldOfView _camera (Math|Interpolation|FInterpTo (Variables|/Script/Engine.CameraComponent|GetFieldOfView _camera) 75.0 (Utilities|Time|GetWorldDeltaSeconds) 8.0))
    (Utilities|Time|ClearandInvalidateTimerbyHandle (Variables|Default|GetOutFOVHandle)))
  (:Completed
    (Variables|Default|SetWant%20To%20Aim false)
    (bind _returnvalue (Utilities|Time|SetTimerbyEvent (delegate Custom|OutFOV) (Utilities|Time|GetWorldDeltaSeconds) true))
    (Variables|Default|SetOutFOVHandle _returnvalue)))

(event Input|EnhancedActionEvents|EnhancedInputActionIA_Fire
  (params (ActionValue :type Boolean) (ElapsedSeconds :type Float%20%28double-precision%29) (TriggeredSeconds :type Float%20%28double-precision%29) (InputAction :type Input%20Action%20Object%20Reference :default "/Game/Code/Player/System/Input/IA_Fire.IA_Fire"))
  (:Started
    (if (not (Variables|Default|GetIsFiring)) ; 如果已经处于开火状态，就不能再执行开火命令了
      (if (not (Variables|Default|GetIsDead))
        (if (Utilities|Enum|NotEqual(Enum) (Variables|Default|GetE_PlayerState) "NewEnumerator2") ; 奔跑状态下不能开火
          (Variables|Default|SetIsFiring true)
          (Class|BIFire|StartWeaponFire(Message) (Variables|Default|GetCurrentWeapon) self)))))
  (:Completed
    (Default|StopFire (Variables|Default|GetCurrentWeapon))
    (Variables|Default|SetIsFiring false)))

(event EventBeginPlay
  (bind _as玩家控制器 (Utilities|Casting|CastToPlayerController (Pawn|GetController)))
  (Input|AddMappingContext (PlayerController|LocalPlayerSubsystems|GetEnhancedInputLocalPlayerSubsystem _as玩家控制器) "/Game/Code/Player/System/Input/IMC_FPSInput.IMC_FPSInput" 0 "(bIgnoreAllPressedKeysUntilRelease=True,bForceImmediately=False,bNotifyUserSettings=False)")
  (CallFunction|SpawnWeapon "/Game/Code/Weapon/BP_VIRTUS.BP_VIRTUS_C")
  (CallFunction|UpdateDefaultFOV))

(event EventTick
  (params (DeltaSeconds :type Float%20%28single-precision%29))
  (bind _returnvalue (Pawn|GetControlRotation :!class /Script/Engine.Pawn))
  (Transformation|SetWorldRotation (Variables|Default|GetArm) (Math|Rotator|MakeRotator 0.0 (.pitch _returnvalue) (.yaw _returnvalue)) false false)
  (CallFunction|UpdatePlayerState)
  (CallFunction|UpdateMoveSpeed)
  (Development|PrintString (Utilities|String|ToString(Float) (Variables|/Script/Engine.CharacterMovementComponent|GetMaxWalkSpeed (Variables|Character|GetCharacterMovement))) true true "(R=0.000000,G=0.660000,B=1.000000,A=1.000000)" 0.0))

(fn ConstructionScript)

(fn UpdatePlayerState
  (if (Variables|Default|GetWant%20To%20Aim) ; 是否按下鼠标右键瞄准
    (Variables|Default|SetE_PlayerState "NewEnumerator3")
    (elif (> (Variables|Default|GetMove%20X) 0.0) ; 是否在X方向上有移动
      (if (Variables|Default|GetWant%20To%20Run) ; 是否按Shift奔跑
        (Variables|Default|SetE_PlayerState "NewEnumerator2")
        (else
          (Variables|Default|SetE_PlayerState "NewEnumerator1")))
      (elif (> (Math|Vector|VectorLength (Variables|/Script/Engine.MovementComponent|GetVelocity (Variables|Character|GetCharacterMovement))) 0.0) ; 是否在其他方向上有移动
        (Variables|Default|SetE_PlayerState "NewEnumerator1")
        (else
          (Variables|Default|SetE_PlayerState "NewEnumerator0"))))))

(fn UpdateMoveSpeed
  (Variables|/Script/Engine.CharacterMovementComponent|SetMaxWalkSpeed (Variables|Character|GetCharacterMovement) (Utilities|Select :Index (Variables|Default|GetE_PlayerState) :NewEnumerator0 4e+02 :NewEnumerator1 4e+02 :NewEnumerator2 6e+02 :NewEnumerator3 265.0)))

(fn SpawnWeapon
  (params (Class :type Actor%20Class%20Reference))
  (bind _returnvalue (Game|SpawnActorfromClass Class (Math|Transform|MakeTransform "0, 0, 0" "0, 0, 0" "1.000000,1.000000,1.000000") "Undefined" "MultiplyWithRoot" self 0))
  (bind _asbp_weapon_base (Utilities|Casting|CastToBP_WeaponBase _returnvalue))
  (bind _output_get (Variables|Default|SetCurrentWeapon _asbp_weapon_base))
  (Transformation|AttachComponentToComponent _output_get (Variables|Default|GetArm) "None" "KeepRelative" "KeepRelative" "KeepRelative" true))

(fn UpdateDefaultFOV
  (Variables|Default|SetDefaultFOV (Variables|/Script/Engine.CameraComponent|GetFieldOfView (Variables|Default|GetCamera))))

(fn UpdateScopeSensitivity
  (return (Utilities|Select :Index (Variables|Default|GetE_PlayerState) :NewEnumerator0 1.0 :NewEnumerator1 1.0 :NewEnumerator2 1.0 :NewEnumerator3 0.4)))
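; BP_WeaponBase is a base weapon Blueprint that handles automatic-fire animation and exposes the weapon's aim socket location.
; StartWeaponFire stores the player, checks ammo once, fires immediately, then repeats FireInternal on a looping FireRate timer until StopFire clears it.
; Each shot plays a weapon montage, then an arm montage, selected by player state, with none set for Run.
; Ammo consumption and hit logic are absent here.
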(event Custom|FireInternal
  (Animation|Montage|PlayMontage (Variables|Default|GetWeapon) (Utilities|Select :Index (Variables|/Game/Code/Player/BP_FPSPlayer.BP_FPSPlayer_C|GetE_PlayerState (Variables|Default|GetPlayer)) :NewEnumerator0 (Variables|Default|GetWeapon_Idle) :NewEnumerator1 (Variables|Default|GetWeapon_Walk) :NewEnumerator2 0 :NewEnumerator3 (Variables|Default|GetWeapon_Aim))
    (:then
      (Animation|Montage|PlayMontage (Variables|/Game/Code/Player/BP_FPSPlayer.BP_FPSPlayer_C|GetArm (Variables|Default|GetPlayer)) (Utilities|Select :Index (Variables|/Game/Code/Player/BP_FPSPlayer.BP_FPSPlayer_C|GetE_PlayerState (Variables|Default|GetPlayer)) :NewEnumerator0 (Variables|Default|GetPlayer_Idle) :NewEnumerator1 (Variables|Default|GetPlayer_Walk) :NewEnumerator2 0 :NewEnumerator3 (Variables|Default|GetPlayer_Aim))))))

(event Custom|StopFire
  (Utilities|Time|ClearandInvalidateTimerbyHandle (Variables|Default|GetFireTimerHandle)))

(event EventBeginPlay)

(event Collision|EventActorBeginOverlap
  (params (OtherActor :type Actor%20Object%20Reference)))

(event EventTick
  (params (DeltaSeconds :type Float%20%28single-precision%29)))

(event EventStartWeaponFire
  (params (Player :type BP%20FPS%20Player%20Object%20Reference))
  (Variables|Default|SetPlayer Player)
  (if (> (Variables|Default|GetCurrentAmmo) 0)
    (CallFunction|FireInternal)
    (bind _returnvalue (Utilities|Time|SetTimerbyEvent (delegate Custom|FireInternal) (Variables|Default|GetFireRate) true))
    (Variables|Default|SetFireTimerHandle _returnvalue)))

(fn ConstructionScript)

(fn GetAimSocketLocation
  (bind _output_get (Variables|Default|SetAimSocketLocation (Transformation|GetSocketLocation (Variables|Default|GetWeapon) "AimSocket")))
  (return _output_get))